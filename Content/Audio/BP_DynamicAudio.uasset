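; BP_DynamicAudio plays the game's soundtrack as a 2D MetaSound and exposes an event to change its intensity.
; BeginPlay creates and starts MS_SoundTrack without auto-destroy, keeping the audio component for later parameter changes.
; IntensifyMusic runs the FadeInMusic timeline and selects a volume parameter by intensity level.
; Only level 1 follows the fade curve; levels 2 and 3 set their volume parameters to zero.
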(event Custom|IntensifyMusic
  (params (Intensity :type Integer))
  (bind _metasound (Variables|Default|GetMetaSound))
  (bind _fadeup (Timeline|FadeInMusic PlayFromStart)
    (:Update
      (switch int Intensity
        (:1
          (Audio|Parameter|SetFloatParameter _metasound "Volume1" _fadeup :!class /Script/AudioExtensions.AudioParameterControllerInterface))
        (:2
          (Audio|Parameter|SetFloatParameter _metasound "Volume2" 0.0 :!class /Script/AudioExtensions.AudioParameterControllerInterface))
        (:3
          (Audio|Parameter|SetFloatParameter _metasound "Volume3" 0.0 :!class /Script/AudioExtensions.AudioParameterControllerInterface))))))

(event EventBeginPlay
  (bind _returnvalue (Audio|CreateSound2D "/Game/Audio/MS_SoundTrack.MS_SoundTrack" 1.0 1.0 0.0 0 false false))
  (bind _output_get (Variables|Default|SetMetaSound _returnvalue))
  (Audio|Components|Audio|Play _output_get 0.0)
  (Audio|Components|Audio|AdjustVolume _output_get 0.0 1.0 "Linear" :!class /Script/Engine.AudioComponent))

(fn ConstructionScript)