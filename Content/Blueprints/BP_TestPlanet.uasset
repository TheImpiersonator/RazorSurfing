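; BP_TestPlanet is a test planet actor that gives the third-person character spherical gravity while it overlaps the actor.
; Begin overlap stores the character and sets an on-planet flag.
; While that flag is set, Tick points the character movement's gravity direction toward the planet's origin.
; End overlap restores straight-down gravity and clears the flag.
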(event EventTick
  (params (DeltaSeconds :type Float%20%28single-precision%29))
  (bind _as_bp_third_person_character (Variables|Default|GetAs%20BP%20Third%20Person%20Character))
  (if (Variables|Default|GetIsOnPlanet)
    (Utilities|IsValid _as_bp_third_person_character
      (:Is%20Valid
        (Class|CharacterMovementComponent|SetGravityDirection (Variables|/Script/Engine.Character|GetCharacterMovement _as_bp_third_person_character) (Math|Vector|NegateVector (Math|Vector|Normalize (- (Transformation|GetActorLocation _as_bp_third_person_character) (Transformation|GetActorLocation)))))))))

(event Collision|EventActorBeginOverlap
  (params (OtherActor :type Actor%20Object%20Reference))
  (bind _asbp_third_person_character (Utilities|Casting|CastToBP_ThirdPersonCharacter OtherActor))
  (Variables|Default|SetAs%20BP%20Third%20Person%20Character _asbp_third_person_character)
  (Variables|Default|SetIsOnPlanet true))

(event Collision|EventActorEndOverlap
  (params (OtherActor :type Actor%20Object%20Reference))
  (bind _asbp_third_person_character (Utilities|Casting|CastToBP_ThirdPersonCharacter OtherActor))
  (Class|CharacterMovementComponent|SetGravityDirection (Variables|/Script/Engine.Character|GetCharacterMovement _asbp_third_person_character) (Math|Vector|MakeVector 0.0 0.0 -1.0))
  (Variables|Default|SetIsOnPlanet false))

(fn ConstructionScript)