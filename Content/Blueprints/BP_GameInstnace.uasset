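; BP_GameInstnace tracks whisker hair loss and ends the game in a win once at least 80% of the initial hairs are lost.
; InitHair counts BP_SingleWhisker actors, while BeginPlay binds a hair-destroyed event through BP_SurfingGameMode to increment the loss count.
; Count changes broadcast HairUpdated.
; EndGame freezes the player, passes the result to BP_EndCamera and blends the view to it.
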(event Custom|HairDestroyed_Event
  (CallFunction|HairLoss)
  (Default|CallHairUpdated))

(event Custom|Begin%20Play
  (bind _asbp_surfing_game_mode (Utilities|Casting|CastToBP_SurfingGameMode (Game|GetGameMode)))
  (EventDispatchers|AssignHairDestroyed _asbp_surfing_game_mode (delegate Custom|HairDestroyed_Event)))

(fn CountHairs
  (bind _outactors (Actor|GetAllActorsOfClass "/Game/Blueprints/BP_SingleWhisker.BP_SingleWhisker_C"))
  (bind _output_get (Variables|Default|SetInit_Hairs (Utilities|Array|Length _outactors))))

(fn HairLoss
  (bind _result (Math|Integer|IncrementInt (Variables|Default|GetHairs%20Lost))
    (:%20%20
      (Default|CallHairUpdated)
      (if (>= _result (* (Variables|Default|GetInit_Hairs) 0.8))
        (CallFunction|EndGame true)))))

(fn InitHair
  (CallFunction|CountHairs)
  (Default|CallHairUpdated))

(fn EndGame
  (params (DidWin :type Boolean))
  (bind _asbp_third_person_character (Utilities|Casting|CastToBP_ThirdPersonCharacter (Game|Player|GetPlayerPawn 0)))
  (Default|FreezePlayer _asbp_third_person_character true)
  (bind _returnvalue (Actor|GetActorOfClass "/Game/Blueprints/BP_EndCamera.BP_EndCamera_C"))
  (Default|EndGame _returnvalue DidWin)
  (Game|Player|SetViewTargetwithBlend (Game|GetPlayerController 0) _returnvalue 3.0 "VTBlend_Linear" 0.0 false))