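; BP_SingleWhisker is a single whisker hair in the surfing game that the player destroys by touching it.
; When the player pawn overlaps it, it calls CallHairDestroyed on BP_SurfingGameMode and destroys itself.
; Its construction script adds a random local rotation with slight pitch and roll and full yaw, so placed whiskers vary in orientation.
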(event Collision|EventActorBeginOverlap
  (params (OtherActor :type Actor%20Object%20Reference))
  (if (== OtherActor (Game|Player|GetPlayerPawn 0))
    (bind _asbp_surfing_game_mode (Utilities|Casting|CastToBP_SurfingGameMode (Game|GetGameMode)))
    (Default|CallHairDestroyed _asbp_surfing_game_mode)
    (Actor|DestroyActor)))

(fn ConstructionScript
  (Transformation|AddActorLocalRotation (Math|Rotator|MakeRotator (Math|Random|RandomFloatinRange -2e+01 2e+01) (Math|Random|RandomFloatinRange -2e+01 2e+01) (Math|Random|RandomFloatinRange 0.0 3.6e+02)) false false))